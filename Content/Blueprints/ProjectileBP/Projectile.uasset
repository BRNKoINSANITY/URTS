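; Projectile Blueprint meant to fire a configurable shell from a gun location toward a target, with an optional artillery arc.
; BeginPlay calculates a suggested toss velocity, then adds sphere collision, projectile movement and child actor components at runtime.
; Hit destroys those components and adds a child actor at the impact point for the effect.
; The nodes setting velocity, bullet model and impact model are unwired, so none are applied.
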(event EventBeginPlay
  (bind _gun_location (Variables|Default|Getgun%20location))
  (bind _bullet_size (Variables|Default|Getbullet%20size))
  ;[1 1 1] Calculates trajectory of future projectile, then creates a collision sphere and movement component. Attaches projectile model to the movement and collision components, and launches the projectile on recommended trajectory.
  (bind _tossvelocity (Class|GameplayStatics|BlueprintSuggestProjectileVelocity _gun_location (Variables|Default|Gettarget%20location) (Variables|Default|Getbullet%20speed) 0.0 "DoNotTrace" (Variables|Default|Getbullet%20circumference) (Variables|Default|Getartillery%20trajectory) false))
  (bind _returnvalue (AddComponent|AddSphereComponent false (Math|Transform|MakeTransform _gun_location "0, 0, 0" _bullet_size)))
  (bind _returnvalue_2 (AddComponent|AddProjectileMovementComponent))
  (bind _returnvalue_3 (AddComponent|AddChildActorComponent false (Math|Transform|MakeTransform _gun_location "0, 0, 0" _bullet_size))))

(event Collision|EventHit
  (params (MyComp :type Primitive%20Component%20Object%20Reference) (Other :type Actor%20Object%20Reference) (OtherComp :type Primitive%20Component%20Object%20Reference) (bSelfMoved :type Boolean) (HitLocation :type Vector :default "0, 0, 0") (HitNormal :type Vector :default "0, 0, 0") (NormalImpulse :type Vector :default "0, 0, 0") (Hit :type Hit%20Result%20Structure%20%28by%20ref%29))
  ;[1 1 1] On collision, deletes all created actors and spawns the chosen impact effect.
  (Components|DestroyComponent (stale EventBeginPlay _returnvalue_3))
  (bind _returnvalue (AddComponent|AddChildActorComponent false (Math|Transform|MakeTransform HitLocation "0, 0, 0" (Variables|Default|Getbullet%20impact%20size)))))

(fn ConstructionScript)